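; Multi-mode defense gun combining a gravity gun with add-on mods that damage Robots, with shock or freeze by mod type.
; Mode 0 pushes or launches pickUpable objects, while Fire2 grabs or releases them.
; UpdateData refreshes muzzle and forward points for line traces and beam particles, pinning any held object at the forward point.
; AddMod registers each mod's particles and sounds, with Mode indexing sounds directly and mods offset by one.
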(event EventFire
  (CallFunction|PowerUp)
  (if (== (Variables|Default|GetMode) 0)
    ;[1 1 1] D-Mode one
    (if (Variables|Default|GetholdObject)
      ;;[1 1 1] Launch
      (bind _finalforce (CallFunction|CalculateForce (Variables|Default|GetholdingObj)))
      (Default|AddNewForce (Variables|Default|GetholdingObj) _finalforce)
      ;;[1 1 1] Realease
      (Default|SetGravity (Variables|Default|GetholdingObj) true)
      (Variables|Default|SetholdingObj 0)
      (Variables|Default|SetholdObject false)
      (else
        ;;[1 1 1] Push
        (bind (_hit _actor) (CallFunction|TraceOut))
        (if _hit
          (bind _aspickupable_c (Utilities|Casting|CastTopickUpable _actor))
          (bind _finalforce_2 (CallFunction|CalculateForce _aspickupable_c))
          (Default|AddNewForce _aspickupable_c _finalforce_2))))
    (else
      (Variables|Default|Setfireing true)
      (bind _hit_2 (CallFunction|TraceOut))
      (if _hit_2
        ;[1 1 1] modes Two and up Hit
        (bind _asrobot_c (Utilities|Casting|CastToRobot (Variables|Default|GetActorHit))
          (:then
            (bind _mod (CallFunction|GetMod))
            (Components|Activation|SetActive (Variables|/Game/Blueprints/Guns/GunMods/Deffence/DeffenceMod.DeffenceMod_C|GetParticleSystem _mod) true false)
            (Default|TakeDamage _asrobot_c (Variables|/Game/Blueprints/Guns/GunMods/Deffence/DeffenceMod.DeffenceMod_C|GetDamage _mod))
            (if (== (Variables|/Game/Blueprints/Guns/GunMods/Deffence/DeffenceMod.DeffenceMod_C|GetType _mod) 0)
              (Default|SystemShock _asrobot_c)
              (Development|PrintString "Electric" true true "(R=0.040000,G=1.000000,B=0.171507,A=1.000000)")
              (elif (== (Variables|/Game/Blueprints/Guns/GunMods/Deffence/DeffenceMod.DeffenceMod_C|GetType _mod) 1)
                (Default|FreezeUp _asrobot_c)
                (Development|PrintString "Freeze" true true "(R=0.040000,G=1.000000,B=0.171507,A=1.000000)"))))
          (:CastFailed
            ;[1 1 1] Fire anyway
            (bind _mod_2 (CallFunction|GetMod :!label _label))
            (Components|Activation|SetActive (Variables|/Game/Blueprints/Guns/GunMods/Deffence/DeffenceMod.DeffenceMod_C|GetParticleSystem _mod_2) true false)))
        (else
          (goto _label))))))

(event EventFire2
  ;[1 1 1] D-Mode one
  (if (Variables|Default|GetholdObject)
    ;;[1 1 1] Realease
    (Default|SetGravity (Variables|Default|GetholdingObj) true)
    (Variables|Default|SetholdingObj 0)
    (Variables|Default|SetholdObject false)
    (else
      ;;[1 1 1] Grab
      (bind (_hit _actor) (CallFunction|TraceOut))
      (if _hit
        (bind _aspickupable_c (Utilities|Casting|CastTopickUpable _actor))
        (Variables|Default|SetholdingObj _aspickupable_c)
        (Default|NewLocation (Variables|Default|GetholdingObj) (Variables|Default|GetForward))
        (Default|SetGravity (Variables|Default|GetholdingObj) false)
        (Variables|Default|SetholdObject true)
        (Variables|/Game/InteractibleObjects/pickUpable.pickUpable_C|SetinAir (Variables|Default|GetholdingObj) true)))))

(event EventRealease
  (Variables|Default|Setfireing false)
  (CallFunction|PowerDown)
  (for _array_element (Variables|Default|GetDefenceMods)
    (Components|Activation|Deactivate (Variables|/Game/Blueprints/Guns/GunMods/Deffence/DeffenceMod.DeffenceMod_C|GetParticleSystem _array_element))))

(event EventUpdateData
  (bind _holdingobj (Variables|Default|GetholdingObj))
  (CallFunction|Update)
  ;[1 1 1] D-Mode one
  (if (Variables|Default|GetholdObject)
    ;;[1 1 1] Holding
    (Default|NewLocation _holdingobj (Variables|Default|GetForward))
    (Default|SetForces _holdingobj "0, 0, 0" "0, 0, 0" false)
    (Default|SetRotation _holdingobj (Transformation|GetWorldRotation (Variables|Default|GetMuzzel)))))

(event EventSetPhysics
  (params (On :type Boolean))
  (bind _g2 (Variables|Default|Getg2))
  (Physics|SetEnableGravity _g2 On)
  (Physics|SetSimulatePhysics _g2 On))

(fn ConstructionScript
  (|CallParentFunction)
  (Variables|Default|SetMax 1)
  (Variables|Default|SetDistance 3e+02)
  (Variables|Default|SetForce 1e+03)
  (Variables|Default|Setfireing false)
  (CallFunction|SetAudio))

(fn Update
  (bind _muzzel (Variables|Default|GetMuzzel))
  (bind _returnvalue (Transformation|GetWorldLocation _muzzel))
  (Variables|Default|SetMuzzelLocat _returnvalue)
  (Variables|Default|SetForward (+ _returnvalue (* (Math|Vector|GetForwardVector _muzzel) (Variables|Default|GetDistance))))
  (for _array_element (Variables|Default|GetDefenceMods)
    (Class|ParticleSystemComponent|SetBeamTargetPoint (Variables|/Game/Blueprints/Guns/GunMods/Deffence/DeffenceMod.DeffenceMod_C|GetParticleSystem _array_element) 0 (Variables|Default|GetForward))
    (Class|ParticleSystemComponent|SetBeamSourcePoint (Variables|/Game/Blueprints/Guns/GunMods/Deffence/DeffenceMod.DeffenceMod_C|GetParticleSystem _array_element) 0 (Variables|Default|GetMuzzelLocat))))

(fn CalculateForce
  (params (object :type Actor%20Object%20Reference))
  (return (Math|Vector|RotateVector (* (Transformation|GetActorLocation object) (Variables|Default|GetForce)) (Math|Rotator|FindLookatRotation (Variables|Default|GetForward) (Variables|Default|GetMuzzelLocat)))))

(fn TraceOut
  (bind (_outhit _returnvalue) (Collision|LineTraceByChannel (Variables|Default|GetMuzzelLocat) (Variables|Default|GetForward) "TraceTypeQuery2" false 0 "ForDuration"))
  (Variables|Default|SetActorHit (.HitActor (Collision|BreakHitResult _outhit)))
  (return _returnvalue (.HitActor (Collision|BreakHitResult _outhit))))

(fn AddMod
  (params (newMod :type Deffence%20Mod%20Object%20Reference))
  (CallFunction|AddSounds newMod)
  (Utilities|Array|Add (Variables|Default|GetDefenceMods) newMod)
  (Default|CreateSystem newMod (Variables|Default|GetMuzzel))
  (Variables|Default|SetMax (+ 1 (Variables|Default|GetMax))))

(fn GetMod
  (bind _mode (Variables|Default|GetMode))
  (bind _defencemods (Variables|Default|GetDefenceMods))
  (bind _returnvalue (- _mode 1))
  (bind _item (Utilities|Array|Get(acopy) _defencemods _returnvalue))
  (Development|PrintString (Utilities|String|Append "Get Mod Valid: " (Utilities|String|ToString(Boolean) (Utilities|IsValid _item))))
  (return _item))

(fn PowerUp
  (CallFunction|SetSounds)
  (Audio|Components|Audio|Play (Variables|Default|Getstartup) 0.0)
  (Audio|Components|Audio|Play (Variables|Default|Getambient) 0.0))

(fn SetSounds
  (bind _mode (Variables|Default|GetMode))
  ;[1 1 1] Take 3
  (Audio|Components|Audio|SetSound (Variables|Default|Getambient) (Utilities|Array|Get(acopy) (Variables|Default|GetHumSounds) _mode))
  (Audio|Components|Audio|SetSound (Variables|Default|Getstartup) (Utilities|Array|Get(acopy) (Variables|Default|GetPowerUpSounds) _mode))
  (Audio|Components|Audio|SetSound (Variables|Default|Getshutdown) (Utilities|Array|Get(acopy) (Variables|Default|GetPowerDownSounds) _mode)))

(fn PowerDown
  (Audio|Components|Audio|Play (Variables|Default|Getshutdown) 0.0)
  (Audio|Components|Audio|Stop (Variables|Default|Getambient))
  (Audio|Components|Audio|Stop (Variables|Default|Getstartup)))

(fn SetAudio
  ;[1 1 1] Take 3
  (Utilities|Array|Add (Variables|Default|GetHumSounds) "/Game/Blueprints/Guns/Sounds/Defense/Gravity/Hum.Hum")
  (Utilities|Array|Add (Variables|Default|GetPowerUpSounds) "/Game/Blueprints/Guns/Sounds/Defense/Gravity/powerupGravity.powerupGravity")
  (Utilities|Array|Add (Variables|Default|GetPowerDownSounds) "/Game/Blueprints/Guns/Sounds/Defense/Gravity/PowerDownGravity.PowerDownGravity"))

(fn AddSounds
  (params (NewMod :type Deffence%20Mod%20Object%20Reference))
  (Utilities|Array|Add (Variables|Default|GetHumSounds) (Variables|/Game/Blueprints/Guns/GunMods/Deffence/DeffenceMod.DeffenceMod_C|GetHum NewMod))
  (Utilities|Array|Add (Variables|Default|GetPowerUpSounds) (Variables|/Game/Blueprints/Guns/GunMods/Deffence/DeffenceMod.DeffenceMod_C|GetPowerUp NewMod))
  (Utilities|Array|Add (Variables|Default|GetPowerDownSounds) (Variables|/Game/Blueprints/Guns/GunMods/Deffence/DeffenceMod.DeffenceMod_C|GetPowerDown NewMod)))