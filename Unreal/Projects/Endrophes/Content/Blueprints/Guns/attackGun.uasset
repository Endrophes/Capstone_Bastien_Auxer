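; Gun Blueprint that spawns the current mode's bullet just ahead of the muzzle, toggling the muzzle flash and playing that mode's sound.
; Parallel bullet, sound and icon arrays start with a Standard entry and grow through AddMod, with Mode indexing the bullet and sound.
; FireinGeneralDirection offsets the spawn along a given direction but keeps the gun mesh's rotation.
; SetPhysics toggles gravity and simulation on the mesh.
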(event `self.setPhysics`
  (params (On :type Boolean))
  (bind _g1 (`self.g1`))
  (`PrimitiveComponent.SetEnableGravity` _g1 On)
  (`PrimitiveComponent.SetSimulatePhysics` _g1 On))

(event `self.Fire`
  (`ActorComponent.ToggleActive` (`self.muzzleFlash`))
  (`self.PlayCue`)
  (bind _selected (`self.get Bullet`))
  (bind _bullettransform (`self.Get Transform for Bullet`))
  (`|SpawnActorFromClass` _selected _bullettransform true))

(event `self.Fire in general Direction`
  (params (direction :type "Object.Vector Structure"))
  (`ActorComponent.ToggleActive` (`self.muzzleFlash`))
  (`self.PlayCue`)
  (bind _final_transform (`self.get transform from Direction` direction))
  (bind _selected (`self.get Bullet`))
  (`|SpawnActorFromClass` _selected _final_transform true))

(event `self.UpdateData`)

(fn `Add Mod`
  (params (NewMod :type "/Game/Blueprints/Guns/GunMods/Attack/AttackMod Object Reference"))
  (`KismetArrayLibrary.Array_Add` (`self.BulletSet`) (`/Game/Blueprints/Guns/GunMods/Attack/AttackMod.BulletType` NewMod))
  (`KismetArrayLibrary.Array_Add` (`self.bulletSounds`) (`/Game/Blueprints/Guns/GunMods/Attack/AttackMod.sound` NewMod))
  (`KismetArrayLibrary.Array_Add` (`self.ModeIcon`) (`/Game/Blueprints/Guns/GunMods/Attack/AttackMod.Icon` NewMod)))

(fn `get Bullet`
  (returns (selected :type "Actor Class Reference"))
  (return (`KismetArrayLibrary.Array_Get` (`self.BulletSet`) (`self.Mode`))))

(fn `Get Transform for Bullet`
  (returns (BulletTransform :type "Object.Transform Structure"))
  (bind _muzzle (`self.Muzzle`))
  (return (`KismetMathLibrary.MakeTransform` (+ (`SceneComponent.K2_GetComponentLocation` _muzzle) (* (`SceneComponent.GetForwardVector` _muzzle) 10.0)) (`SceneComponent.K2_GetComponentRotation` (`self.g1`)))))

(fn `get transform from Direction`
  (params (`Forward Direction` :type "Object.Vector Structure"))
  (returns (`final transform` :type "Object.Transform Structure"))
  (return (`KismetMathLibrary.MakeTransform` (+ (`SceneComponent.K2_GetComponentLocation` (`self.Muzzle`)) (* `Forward Direction` 10.0)) (`SceneComponent.K2_GetComponentRotation` (`self.g1`)))))

(fn `PlayCue`
  (bind _ambient (`self.ambient`))
  (`AudioComponent.SetSound` _ambient (`KismetArrayLibrary.Array_Get` (`self.bulletSounds`) (`self.Mode`)))
  (`AudioComponent.Play` _ambient 0.0))

(fn `Set Up Sound Array`
  (`KismetArrayLibrary.Array_Add` (`self.bulletSounds`) "/Game/Blueprints/Guns/Sounds/Attack/Standard.Standard"))

(fn `setUpBulletArray`
  (bind _bulletset (`self.BulletSet`))
  (`KismetArrayLibrary.Array_Add` _bulletset "/Game/Blueprints/Bullets/standard.standard_C")
  (set `self.Max` (`KismetArrayLibrary.Array_Length` _bulletset)))

(fn `UserConstructionScript`
  (`parent.UserConstructionScript`)
  (set `self.UseData` true)
  (set `self.Mode` 0)
  (`self.setUpBulletArray`)
  (`self.Set Up Sound Array`)
  (`KismetArrayLibrary.Array_Add` (`self.ModeIcon`) "/Game/Blueprints/UI/Texture/Icons/Attack/Standard/Bullet/StandardIcon.StandardIcon"))