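; Base gun Blueprint that defines a common interface for weapons with selectable modes.
; SelectMode steps Mode up or down with wraparound below Max, does nothing to it when Max is zero, and prints the result on screen.
; Construction resets the mode state and UseData flag, while primary and secondary fire, release, data update and physics toggle functions are empty stubs.
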(fn ConstructionScript
  (Variables|Default|SetMode 0)
  (Variables|Default|SetMax 0)
  (Variables|Default|SetUseData false))

(fn SelectMode
  (params (up :type Boolean))
  (bind _max (Variables|Default|GetMax))
  ;[1 1 1] DoubleCheck
  (if (== (Variables|Default|GetMax) 0)
    _
    (elif up
      ;[1 1 1] Up
      (if (>= (+ (Variables|Default|GetMode) 1) _max)
        (Variables|Default|SetMode 0)
        (else
          (Variables|Default|SetMode (+ (Variables|Default|GetMode) 1))))
      (else
        ;[1 1 1] Down
        (if (< (- (Variables|Default|GetMode) 1) 0)
          (Variables|Default|SetMode (- _max 1))
          (else
            (Variables|Default|SetMode (- (Variables|Default|GetMode) 1)))))))
  (Development|PrintString (Utilities|String|ToString(Integer) (Variables|Default|GetMode)) true true "(R=1.000000,G=0.785793,B=0.000000,A=1.000000)"))

(fn Fire)

(fn Fire2)

(fn Realease)

(fn UpdateData)

(fn SetPhysics
  (params (On :type Boolean)))