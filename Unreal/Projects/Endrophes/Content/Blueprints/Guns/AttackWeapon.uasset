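; AttackWeapon is a gun Blueprint that spawns one of several bullet types based on the selected mode.
; The construction script fills BulletSet with Standard, NewRicochet and HighX classes, and scroll input cycles Mode through it with wraparound.
; Fire, which has no caller in this graph, spawns the selected class at a supplied location and rotation unless colliding.
; Debug strings print on mode changes and firing.
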(event Input|ActionEvents|InputActionScrollUp
  ;[1 1 1] Set Mode
  (:Pressed
    (CallFunction|SetMode true)
    (Development|PrintString (Utilities|String|ToString(Integer) (Variables|Default|GetMode)) true true "(R=1.000000,G=0.931485,B=0.101279,A=1.000000)")))

(event Input|ActionEvents|InputActionScrollDown
  ;[1 1 1] Set Mode
  (:Pressed
    (CallFunction|SetMode false)
    (Development|PrintString (Utilities|String|ToString(Integer) (Variables|Default|GetMode)) true true "(R=1.000000,G=0.931485,B=0.101279,A=1.000000)")))

(fn ConstructionScript
  (bind _bulletset (Variables|Default|GetBulletSet))
  (Variables|Default|SetMode 0)
  (Utilities|Array|Add _bulletset "/Game/Blueprints/Bullets/standard.standard_C")
  (Utilities|Array|Add _bulletset "/Game/Blueprints/Bullets/NewRicochet.NewRicochet_C")
  (Utilities|Array|Add _bulletset "/Game/Blueprints/Bullets/highX.highX_C"))

(fn GetBullet
  (return (Utilities|Array|Get(acopy) (Variables|Default|GetBulletSet) (Variables|Default|GetMode))))

(fn Fire
  (params (Location :type Vector) (Rotation :type Rotator))
  (Development|PrintString "Select" true true "(R=0.079946,G=0.194840,B=1.000000,A=1.000000)")
  (bind _selected (CallFunction|GetBullet))
  (Development|PrintString "Spawn" true true "(R=0.143215,G=1.000000,B=0.122903,A=1.000000)")
  (Game|SpawnActorfromClass _selected (Math|Transform|MakeTransform Location Rotation) false))

(fn SetMode
  (params (Up :type Boolean))
  (LocalVariables|SetMax (Utilities|Array|Length (Variables|Default|GetBulletSet)))
  (if Up
    ;[1 1 1] Up
    (if (>= (+ (Variables|Default|GetMode) 1) (LocalVariables|GetMax))
      (LocalVariables|SetResult 0)
      (else
        (LocalVariables|SetResult (+ (Variables|Default|GetMode) 1))))
    (else
      ;[1 1 1] Down
      (if (< (- (Variables|Default|GetMode) 1) 0)
        (LocalVariables|SetResult (- (LocalVariables|GetMax) 1))
        (else
          (LocalVariables|SetResult (- (Variables|Default|GetMode) 1))))))
  (Variables|Default|SetMode (LocalVariables|GetResult)))