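; Defense gun that fires a continuous beam to damage Robots, with each mode backed by a DefenseMod actor.
; BeginPlay spawns the starting mod; the current mod supplies particle beam, sounds, icon and damage, though mode 0 uses HeatDamage.
; While firing, Tick line-traces forward, damages the hit Robot and updates the beam endpoint.
; Lift grab, push and launch helpers and shock/freeze logic remain, but nothing live calls them.
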(event EventFire2)

(event EventRealease
  (CallFunction|Deactivate))

(event EventFire
  (CallFunction|Activate))

(event EventSetPhysics
  (params (On :type Boolean)))

(event EventTick
  (params (DeltaSeconds :type Float%20%28single-precision%29))
  (CallFunction|Update))

(event EventBeginPlay
  (CallFunction|AddDefualtMode))

(fn ConstructionScript
  (|CallParentFunction)
  (Variables|Default|SetMax 1)
  (Variables|Default|SetDistance 1e+04)
  (Variables|Default|SetForce 1e+03)
  (Variables|Default|Setfireing false))

(fn Update
  (if (Variables|Default|Getfireing)
    (CallFunction|Trace)
    (bind _mod (CallFunction|GetMod))
    (CallFunction|SetPointsOfBeam (Variables|/Game/Blueprints/Guns/GunMods/Defense/DefenseMod.DefenseMod_C|GetParticleSystem _mod))))

(fn CalculateForce
  (params (object :type Actor%20Object%20Reference))
  (return (Math|Vector|RotateVector (* (Transformation|GetActorLocation object) (Variables|Default|GetForce)) (Math|Rotator|FindLookatRotation (Variables|Default|GetBeam%20End) (Variables|Default|GetBeam%20Start)))))

(fn TraceOut
  (bind (_outhit _returnvalue) (Collision|LineTraceByChannel (Variables|Default|GetBeam%20Start) (Variables|Default|GetBeam%20End) "TraceTypeQuery2" false 0 "ForDuration"))
  (return _returnvalue (.HitActor (Collision|BreakHitResult _outhit))))

(fn AddMod
  (params (newMod :type Defense%20Mod%20Object%20Reference))
  (Utilities|Array|Add (Variables|Default|GetDefenceMods) newMod)
  (Default|CreateSystem newMod (Variables|Default|GetMuzzel))
  (Variables|Default|SetMax (+ 1 (Variables|Default|GetMax))))

(fn GetMod
  (return (Utilities|Array|Get(acopy) (Variables|Default|GetDefenceMods) (Variables|Default|GetMode))))

(fn PowerUp
  (Audio|Components|Audio|Play (Variables|Default|Getstartup) 0.0)
  (Audio|Components|Audio|Play (Variables|Default|Getambient) 0.0))

(fn SetSounds
  (bind _defencemods (Variables|Default|GetDefenceMods))
  (bind _mode (Variables|Default|GetMode))
  (bind _item (Utilities|Array|Get(acopy) _defencemods _mode))
  (LocalVariables|SetStart (Variables|/Game/Blueprints/Guns/GunMods/Defense/DefenseMod.DefenseMod_C|GetHum _item))
  (LocalVariables|SetHum (Variables|/Game/Blueprints/Guns/GunMods/Defense/DefenseMod.DefenseMod_C|GetPowerUp _item))
  (LocalVariables|SetEnd (Variables|/Game/Blueprints/Guns/GunMods/Defense/DefenseMod.DefenseMod_C|GetPowerDown _item))
  (Audio|Components|Audio|SetSound (Variables|Default|Getambient) (LocalVariables|GetHum))
  (Audio|Components|Audio|SetSound (Variables|Default|Getstartup) (LocalVariables|GetStart))
  (Audio|Components|Audio|SetSound (Variables|Default|Getshutdown) (LocalVariables|GetEnd)))

(fn PowerDown
  (Audio|Components|Audio|Play (Variables|Default|Getshutdown) 0.0)
  (Audio|Components|Audio|Stop (Variables|Default|Getambient))
  (Audio|Components|Audio|Stop (Variables|Default|Getstartup)))

(fn CheckTarget
  (params (Object :type Object%20Object%20Reference))
  (Variables|Default|SetholdObject true)
  (bind _aslift_c (Utilities|Casting|CastToLift Object))
  (Variables|Default|SetTarget _aslift_c)
  (Default|NewLocation (Variables|Default|GetTarget) (Variables|Default|GetBeam%20End))
  (Default|SetPhysics (Variables|Default|GetTarget) false))

(fn Release
  (Default|SetPhysics (Variables|Default|GetTarget) true)
  (Variables|Default|SetTarget 0)
  (Variables|Default|SetholdObject false))

(fn UpdateHolding
  (Default|NewLocation (Variables|Default|GetTarget) (Variables|Default|GetBeam%20End)))

(fn Launch
  (bind _target (Variables|Default|GetTarget))
  (bind _finalforce (CallFunction|CalculateForce _target))
  (Default|AddForce _target _finalforce)
  (Default|SetPhysics _target true))

(fn Push
  (bind (_hit _actor) (CallFunction|TraceOut))
  (if _hit
    (bind _aslift_c (Utilities|Casting|CastToLift _actor))
    (bind _finalforce (CallFunction|CalculateForce _aslift_c))
    (Default|AddForce _aslift_c _finalforce)))

(fn Grab
  (bind (_hit _actor) (CallFunction|TraceOut))
  (if _hit
    (CallFunction|CheckTarget _actor)))

(fn ActivateSystem
  (bind _mod (CallFunction|GetMod))
  (Components|Activation|SetActive (Variables|/Game/Blueprints/Guns/GunMods/Defense/DefenseMod.DefenseMod_C|GetParticleSystem _mod) true false))

(fn CheckHit
  (params (Actor :type Object%20Object%20Reference))
  (bind _asrobot_c (Utilities|Casting|CastToRobot Actor))
  (LocalVariables|SetRobot _asrobot_c)
  (if (== (Variables|Default|GetMode) 0)
    (Default|TakeDamage (LocalVariables|GetRobot) (Variables|Default|GetHeatDamage))
    (else
      (bind _mod (CallFunction|GetMod))
      (Default|TakeDamage (LocalVariables|GetRobot) (Variables|/Game/Blueprints/Guns/GunMods/Defense/DefenseMod.DefenseMod_C|GetDamage _mod)))))

(fn Activate
  (Variables|Default|Setfireing true)
  (CallFunction|SetSounds)
  (CallFunction|PowerUp)
  (CallFunction|ActivateSystem))

(fn Deactivate
  (Variables|Default|Setfireing false)
  (CallFunction|PowerDown)
  (for _array_element (Variables|Default|GetDefenceMods)
    (Components|Activation|Deactivate (Variables|/Game/Blueprints/Guns/GunMods/Defense/DefenseMod.DefenseMod_C|GetParticleSystem _array_element))))

(fn Trace
  (bind _tracestart (Variables|Default|GetTraceStart))
  (bind _returnvalue (Transformation|GetWorldLocation _tracestart))
  (Variables|Default|SetBeam%20Start (Transformation|GetWorldLocation (Variables|Default|GetMuzzel)))
  (LocalVariables|Setstart _returnvalue)
  (LocalVariables|SetStop (+ _returnvalue (* (Math|Vector|GetForwardVector _tracestart) (Variables|Default|GetDistance))))
  (bind (_outhit _returnvalue_2) (Collision|LineTraceByChannel (LocalVariables|Getstart) (LocalVariables|GetStop) "TraceTypeQuery2" false 0 "ForOneFrame"))
  (if _returnvalue_2
    (Variables|Default|SetBeam%20End (.Location (Collision|BreakHitResult _outhit)))
    (CallFunction|CheckHit (.HitActor (Collision|BreakHitResult _outhit)))
    (else
      (Variables|Default|SetBeam%20End (LocalVariables|GetStop)))))

(fn SetPointsOfBeam
  (params (System :type Particle%20System%20Component%20Object%20Reference))
  (Class|ParticleSystemComponent|SetBeamTargetPoint System 0 (Variables|Default|GetBeam%20End)))

(fn GetIcon
  (return (Variables|/Game/Blueprints/Guns/GunMods/Defense/DefenseMod.DefenseMod_C|GetIcon (Utilities|Array|Get(acopy) (Variables|Default|GetDefenceMods) (Variables|Default|GetMode)))))

(fn AddDefualtMode
  (bind _returnvalue (Game|SpawnActorfromClass (Variables|Default|GetStartingMode) (Transformation|GetWorldTransform (Variables|Default|Getambient)) false))
  (bind _asdefensemod_c (Utilities|Casting|CastToDefenseMod _returnvalue))
  (Default|SetInvisable _asdefensemod_c)
  (CallFunction|AddMod _asdefensemod_c))