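; Standard bullet Blueprint that damages robots on hit and marks other surfaces with a bullet hole.
; The construction script sets a fixed damage amount.
; On hit, it tries casting the struck actor to Robot, then Robot_Standard, and calls TakeDamage on a match.
; Otherwise it logs the failed cast and spawns a decal at the hit location; the bullet destroys itself either way.
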(event `self.ReceiveHit`
  (params (MyComp :type "PrimitiveComponent Object Reference") (Other :type "Actor Object Reference") (OtherComp :type "PrimitiveComponent Object Reference") (bSelfMoved :type Boolean) (HitLocation :type "Object.Vector Structure") (HitNormal :type "Object.Vector Structure") (NormalImpulse :type "Object.Vector Structure") (Hit :type "EngineTypes.HitResult Structure (by ref)"))
  (bind (_location _normal _impactpoint _impactnormal _physmat _hitactor) (`GameplayStatics.BreakHitResult` Hit))
  (bind _asrobot_c (cast `/Game/Blueprints/bot/Robot` _hitactor)
    (:`then`
      (`/Game/Blueprints/bot/Robot.TakeDamage` _asrobot_c (`self.damageDelt`) :!label _label)
      (`/Game/Blueprints/bot/Robot.TakeDamage` (stale _asrobot_standard_c) (`self.damageDelt`)))
    (:`CastFailed`
      (bind _asrobot_standard_c (cast `/Game/Blueprints/bot/Robot_Standard` _hitactor)
        (:`then`
          (goto _label))
        (:`CastFailed`
          (`KismetSystemLibrary.PrintString` "cast Failed" true true (struct :`R` 1.0 :`G` 0.059947 :`B` 0.069496 :`A` 1.0))
          (`GameplayStatics.SpawnDecalAtLocation` "/Game/Decals/BA_bullet_hole_Mat.BA_bullet_hole_Mat" (50.0 50.0 50.0) HitLocation)))))
  (`self.K2_DestroyActor`))

(fn `UserConstructionScript`
  (set `self.damageDelt` 10.0))