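; Cannon projectile that damages robots and explodes on contact with any overlapping actor.
; On overlap, CheckHit casts the other actor to Robot and applies DamageAmount, then the shot spawns an impact particle at its location and destroys itself.
; The emitter is spawned with auto-destroy off.
; A similar damage branch for MyCharacter exists in CheckHit but is disconnected, so only robots take damage.
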(event `self.ReceiveActorBeginOverlap`
  (params (OtherActor :type "Actor Object Reference"))
  (`self.Check Hit` OtherActor)
  (`GameplayStatics.SpawnEmitterAtLocation` "/Game/Blueprints/Guns/WeaponsOfChoice/Dark/FX/Particles/P_Cannon_Impact_BA.P_Cannon_Impact_BA" (`self.K2_GetActorLocation`) (struct) false)
  (`self.K2_DestroyActor`))

(fn `Check Hit`
  (params (target :type "Object Object Reference"))
  (bind _asrobot_c (cast `/Game/Blueprints/bot/Robot` target))
  (`/Game/Blueprints/bot/Robot.TakeDamage` _asrobot_c (`self.DamageAmount`)))

(fn `UserConstructionScript`)