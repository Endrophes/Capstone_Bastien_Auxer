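; Ricocheting bullet projectile that damages Robot or MyCharacter actors and bounces off anything else.
; On Hit it decrements a bounce counter, then destroys itself after damaging a target or exhausting bounces.
; Otherwise, Ricochet turns the actor along its forward vector reflected about the hit normal, but passes projectile velocity back unchanged.
; Tick counts down a lifetime timer that also destroys the bullet.
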(event EventHit
  (params (MyComp :type Primitive%20Component%20Object%20Reference) (Other :type Actor%20Object%20Reference) (OtherComp :type Primitive%20Component%20Object%20Reference) (bSelfMoved :type Boolean) (HitLocation :type Vector :default "0, 0, 0") (HitNormal :type Vector :default "0, 0, 0") (NormalImpulse :type Vector :default "0, 0, 0") (Hit :type Hit%20Result%20Structure%20%28by%20ref%29))
  (bind _returnvalue (Transformation|GetActorTransform))
  (bind (_location _normal _impactpoint _impactnormal _physmat _hitactor) (Collision|BreakHitResult Hit))
  (bind _projectilemovement1 (Variables|Default|GetProjectileMovement1))
  (bind (_location_2 _rotation _scale) (Math|Transform|BreakTransform _returnvalue))
  (CallFunction|DecramentNumHits)
  (bind _death (CallFunction|CheckHit _hitactor))
  (if _death
    (Actor|DestroyActor :!label _label)
    (elif (== (Variables|Default|GetnumHits) 0)
      (goto _label)
      (else
        (bind (_newtransform _newvelocity) (CallFunction|Ricochet _normal (Transformation|GetActorForwardVector) _location_2 _scale _projectilemovement1))
        (Transformation|SetActorTransform _newtransform)
        (Variables|/Script/Engine.MovementComponent|SetVelocity _projectilemovement1 _newvelocity)))))

(event EventTick
  (params (DeltaSeconds :type Float%20%28single-precision%29))
  (Variables|Default|Settime%20delay (- (Variables|Default|Gettime%20delay) DeltaSeconds))
  (if (< (- (Variables|Default|Gettime%20delay) DeltaSeconds) 0.0)
    (Actor|DestroyActor)))

(fn ConstructionScript
  (Variables|Default|SetnumHits 3)
  (Variables|Default|SetdamageDelt 5.0)
  (Variables|Default|Settime%20delay 5.0))

(fn Ricochet
  (params (Normal :type Vector) (Directional :type Vector) (Location :type Vector) (Scale :type Vector) (Object :type Movement%20Component%20Object%20Reference))
  ;[1 1 1] New Transform
  (bind _result (CallFunction|Reflect Normal Directional))
  (LocalVariables|SetnewTran (Math|Transform|MakeTransform Location (Math|Conversions|RotationFromXVector _result) Scale))
  (LocalVariables|SetNewVel (Variables|/Script/Engine.MovementComponent|GetVelocity Object))
  (return (LocalVariables|GetnewTran) (LocalVariables|GetNewVel)))

(fn PrintVector
  (params (Vector%20Print :type Vector) (text%20Color :type Linear%20Color%20Structure) (PrintToScreen :type Boolean) (PrintToLog :type Boolean) (Message :type String))
  (bind (_x _y _z) (Math|Vector|BreakVector Vector%20Print))
  (bind _returnvalue (Utilities|String|ToString(Float) _z))
  (bind _returnvalue_2 (Utilities|String|ToString(Float) _x))
  (bind _returnvalue_3 (Utilities|String|ToString(Float) _y))
  (bind _returnvalue_4 (Utilities|String|Append _returnvalue_2 ", "))
  (bind _returnvalue_5 (Utilities|String|Append _returnvalue_4 _returnvalue_3))
  (bind _returnvalue_6 (Utilities|String|Append _returnvalue_5 ", "))
  (bind _returnvalue_7 (Utilities|String|Append _returnvalue_6 _returnvalue))
  (if (Utilities|Enum|Equal(Enum) Message "")
    (Development|PrintString _returnvalue_7 PrintToScreen PrintToLog text%20Color)
    (else
      (Development|PrintString (Utilities|String|Append (Utilities|String|Append Message ": ") _returnvalue_7) PrintToScreen PrintToLog text%20Color))))

(fn Reflect
  (params (Normal :type Vector) (Directional :type Vector))
  ;[1 1 1] 2 * (dot(d, ~n))
  (LocalVariables|SetDot%20R (* (Math|Vector|DotProduct Directional Normal) 2.0))
  (return (- Directional (* Normal (LocalVariables|GetDot%20R)))))

(fn DecramentNumHits
  (Variables|Default|SetnumHits (- (Variables|Default|GetnumHits) 1)))

(fn CheckHit
  (params (target :type Object%20Object%20Reference))
  (LocalVariables|SetDie false)
  (bind _asrobot_c (Utilities|Casting|CastToRobot target)
    (:then
      (Default|TakeDamage _asrobot_c (Variables|Default|GetdamageDelt))
      (LocalVariables|SetDie true))
    (:CastFailed
      (bind _asmycharacter_c (Utilities|Casting|CastToMyCharacter target)
        (:then
          (Default|TakeDamage _asmycharacter_c (Variables|Default|GetdamageDelt))
          (LocalVariables|SetDie true))
        (:CastFailed
          _))))
  (return (LocalVariables|GetDie)))