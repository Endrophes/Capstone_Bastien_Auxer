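; Bullet actor that ricochets off surfaces and destroys itself on its fifth hit, counted down from a value set in the construction script.
; On each earlier hit, Ricochet reflects the Arrow's forward vector about the hit normal and rotates the actor to match.
; It zeroes the projectile movement's InitialSpeed as a temporary stop, without setting velocity.
; Debug prints trace hits and vectors; an angle-between-vectors helper is unused.
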(event EventHit
  (params (MyComp :type Primitive%20Component%20Object%20Reference) (Other :type Actor%20Object%20Reference) (OtherComp :type Primitive%20Component%20Object%20Reference) (bSelfMoved :type Boolean) (HitLocation :type Vector :default "0, 0, 0") (HitNormal :type Vector :default "0, 0, 0") (NormalImpulse :type Vector :default "0, 0, 0") (Hit :type Hit%20Result%20Structure%20%28by%20ref%29))
  (bind _returnvalue (Transformation|GetActorTransform))
  (bind (_location _rotation _scale) (Math|Transform|BreakTransform _returnvalue))
  (Development|PrintString "Event Hit")
  (Variables|Default|SetnumHits (- (Variables|Default|GetnumHits) 1))
  (if (== (Variables|Default|GetnumHits) 0)
    (Development|PrintString "Die!" true true "(R=1.000000,G=0.059947,B=0.069496,A=1.000000)")
    (Actor|DestroyActor)
    (else
      (Development|PrintString "Richochet" true true "(R=1.000000,G=0.864895,B=0.053586,A=1.000000)")
      (bind _nexttransform (CallFunction|Ricochet (.Normal (Collision|BreakHitResult Hit)) (Math|Vector|GetForwardVector (Variables|Default|GetArrow)) _location _scale))
      (Transformation|SetActorTransform _nexttransform))))

(fn ConstructionScript
  (Development|PrintString "Fire" true true "(R=0.041199,G=1.000000,B=0.041860,A=1.000000)")
  (Variables|Default|SetnumHits 5))

(fn Ricochet
  (params (normal :type Vector) (Directional :type Vector) (Location :type Vector) (scale :type Vector))
  ;[1 1 1] 2 * (dot(d, ~n)) * ~n
  (LocalVariables|SetdotR (* (Math|Vector|DotProduct Directional normal) 2.0))
  ;[1 1 1] Print out
  (CallFunction|PrintVector normal "(R=1.000000,G=0.121991,B=0.895650,A=1.000000)" true true "Normal")
  (CallFunction|PrintVector Directional "(R=1.000000,G=0.121991,B=0.895650,A=1.000000)" true true "Direction")
  (CallFunction|PrintVector (- Directional (* normal (LocalVariables|GetdotR))) "(R=1.000000,G=0.121991,B=0.895650,A=1.000000)" true true "Result")
  ;[1 1 1] make movment Stop [Temp]
  (Variables|/Script/Engine.ProjectileMovementComponent|SetInitialSpeed (Variables|Default|GetProjectileMovement1) 0.0)
  (return (Math|Transform|MakeTransform Location (Math|Conversions|RotationFromXVector (- Directional (* normal (LocalVariables|GetdotR)))) scale)))

(fn PrintVector
  (params (VectorPrint :type Vector :default "0,0,0") (Text%20Color :type Linear%20Color%20Structure) (Print%20to%20Screen :type Boolean) (Print%20to%20Log :type Boolean) (Message :type String))
  (bind (_x _y _z) (Math|Vector|BreakVector VectorPrint))
  (bind _returnvalue (Utilities|String|ToString(Float) _z))
  (bind _returnvalue_2 (Utilities|String|ToString(Float) _x))
  (bind _returnvalue_3 (Utilities|String|ToString(Float) _y))
  (bind _returnvalue_4 (Utilities|String|Append _returnvalue_2 ", "))
  (bind _returnvalue_5 (Utilities|String|Append _returnvalue_4 _returnvalue_3))
  (bind _returnvalue_6 (Utilities|String|Append _returnvalue_5 ", "))
  (bind _returnvalue_7 (Utilities|String|Append _returnvalue_6 _returnvalue))
  (if (Utilities|Enum|Equal(Enum) Message "")
    (Development|PrintString _returnvalue_7 Print%20to%20Screen Print%20to%20Log Text%20Color)
    (else
      (Development|PrintString (Utilities|String|Append (Utilities|String|Append Message ": ") _returnvalue_7) Print%20to%20Screen Print%20to%20Log Text%20Color))))

(fn AngleinBetweenTwoVectors
  (params (a :type Vector) (b :type Vector))
  (return (Class|KismetMathLibrary|DegAcos (Math|Vector|DotProduct (Math|Vector|Normalize a) (Math|Vector|Normalize b)))))