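; HighX is a bullet actor that deals a fixed amount of damage to robots on impact.
; On hit it spawns an explosion emitter, damages the hit Robot, or hides any non-Robot actor it struck, then destroys itself.
; The construction script sets the damage value; a fire debug print wired ahead of it never runs.
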(event `self.ReceiveHit`
  (params (MyComp :type "PrimitiveComponent Object Reference") (Other :type "Actor Object Reference") (OtherComp :type "PrimitiveComponent Object Reference") (bSelfMoved :type Boolean) (HitLocation :type "Object.Vector Structure") (HitNormal :type "Object.Vector Structure") (NormalImpulse :type "Object.Vector Structure") (Hit :type "EngineTypes.HitResult Structure (by ref)"))
  (bind (_location _normal _impactpoint _impactnormal _physmat _hitactor) (`GameplayStatics.BreakHitResult` Hit))
  (`KismetSystemLibrary.PrintString` "Die HighX !!!" true true (struct :`R` 1.0 :`G` 0.059947 :`B` 0.069496 :`A` 1.0))
  (`GameplayStatics.SpawnEmitterAtLocation` "/Game/Particles/P_BA_Explosion.P_BA_Explosion" (.location (`self.GetTransform`)) (.rotation (`self.GetTransform`)))
  (bind _asrobot_c (cast `/Game/Blueprints/bot/Robot` _hitactor)
    (:`then`
      (`/Game/Blueprints/bot/Robot.TakeDamage` _asrobot_c (`self.damageDelt`)))
    (:`CastFailed`
      (`self.SetActorHiddenInGame` _hitactor true)
      (`KismetSystemLibrary.PrintString` "Cast failed: Robot" true true (struct :`R` 0.41 :`A` 1.0))))
  (`self.K2_DestroyActor`))

(fn `UserConstructionScript`
  (set `self.damageDelt` 15.0))