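; Robot character that spawns a Standard actor ahead of itself when it finds an enemy and shows damage, freeze and shock effects.
; SetUp attaches spark emitters, ice actors and electric emitters to numbered mesh sockets.
; Tick sets walk speed, activates sparks by remaining-health thresholds and counts down to switch off shock emitters.
; TakeDamage accumulates damage, FreezeUp grows the ice to a cap, and SystemShock restarts the electric effect.
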(event `self.ReceiveBeginPlay`
  (`self.SetUp`))

(event `EnemyFound_Event`
  (`self.Attack`))

(event `EnemyLost_Event`)

(event `self.ReceiveTick`
  (params (DeltaSeconds :type "Float (single-precision)"))
  (`self.Update`))

(fn `Activate Sparks`
  (for _index (range (`self.CurrentNumSparksToSet`))
    (bind _item (`KismetArrayLibrary.Array_Get` (`self.particleCollection`) _index))
    (if (not (`ActorComponent.IsActive` _item))
      (`ActorComponent.Activate` _item false))))

(fn `Attack`
  (`|SpawnActorFromClass` "/Game/Blueprints/Bullets/standard.standard_C" (`KismetMathLibrary.MakeTransform` (+ (* (`self.GetActorForwardVector`) 101.0) (`self.K2_GetActorLocation`)) (`self.K2_GetActorRotation`))))

(fn `CalculateNumSparksToActivate`
  (bind _totaldamagecantake (`self.totalDamageCanTake`))
  (bind _returnvalue (- _totaldamagecantake (`self.Damage`)))
  (bind _returnvalue_2 (/ _returnvalue _totaldamagecantake))
  (bind _returnvalue_3 (* 100 _returnvalue_2))
  (`KismetSystemLibrary.PrintString` (`KismetStringLibrary.Concat_StrStr` "subtraction: " (`KismetStringLibrary.Conv_DoubleToString` _returnvalue)))
  (`KismetSystemLibrary.PrintString` (`KismetStringLibrary.Concat_StrStr` "percent: " (`KismetStringLibrary.Conv_DoubleToString` _returnvalue_2)))
  (if (<= _returnvalue_3 75.0)
    (set `self.currentNumSparksToSet` (`self.fourthNumSparks`))
    (if (<= _returnvalue_3 50.0)
      (set `self.currentNumSparksToSet` (`self.halfNumSpArks`))
      (if (<= _returnvalue_3 25.0)
        (set `self.currentNumSparksToSet` (`KismetArrayLibrary.Array_Length` (`self.particleCollection`)))))))

(fn `CalculateWalkSpeed`
  (set `CharacterMovementComponent.MaxWalkSpeed` (* (`self.speedRate`) (`self.speedVar`)) (`self.CharacterMovement`)))

(fn `FreezeUp`
  (`KismetSystemLibrary.PrintString` "FREEZE")
  ;[1 1 1] Cap size of ice
  (if (< (`self.scaleIceAmount`) (`self.icescaleCap`))
    ;[1 1 1] increase ice scale
    (set `self.scaleIceAmount` (+ (`self.scaleIceAmount`) 0.2))
    ;[1 1 1] Scale up the size of the ice
    (for _array_element (`self.iceCollection`)
      (`self.SetActorScale3D` _array_element (* (`self.originalIceScale`) (`self.scaleIceAmount`))))))

(fn `Reset System`
  (for _array_element (`self.elctroEffect`)
    (`ActorComponent.Deactivate` _array_element)))

(fn `SetUp`
  (bind _icecollection (`self.iceCollection`))
  (bind _particlecollection (`self.particleCollection`))
  (bind _elctroeffect (`self.elctroEffect`))
  (bind _returnvalue (`KismetArrayLibrary.Array_Length` (`self.particleCollection`)))
  ;[1 1 1] spark setup
  (for _index (range 1 (+ (`self.maxSparks`) 1))
    (bind _returnvalue_2 (`GameplayStatics.SpawnEmitterAttached` "/Game/Particles/P_Sparks2.P_Sparks2" (`self.Mesh`) (`KismetStringLibrary.Conv_StringToName` (`KismetStringLibrary.Concat_StrStr` "spark" (`KismetStringLibrary.Conv_IntToString` _index))) (0.0 0.0 0.0) (struct) "SnapToTarget" false))
    (bind _returnvalue_3 (`KismetArrayLibrary.Array_Add` _particlecollection _returnvalue_2))
    (bind _item (`KismetArrayLibrary.Array_Get` _particlecollection _returnvalue_3))
    (`ActorComponent.Deactivate` _item)
    (`SceneComponent.SetWorldScale3D` _item (`self.startingScale`)))
  (set `self.fourthNumSparks` (* (/ _returnvalue 4) 3))
  (set `self.halfNumSpArks` (/ _returnvalue 2))
  ;[1 1 1] ice setup
  (for _index_2 (range 1 (+ (`self.numIce`) 1))
    (bind _returnvalue_4 (`|SpawnActorFromClass` "/Game/Blueprints/BA_Ice.BA_Ice_C" (`KismetMathLibrary.MakeTransform` (0.0 0.0 0.0) (struct) (`self.originalIceScale`))))
    (bind _returnvalue_5 (`KismetArrayLibrary.Array_Add` _icecollection _returnvalue_4))
    (bind _item_2 (`KismetArrayLibrary.Array_Get` _icecollection _returnvalue_5))
    (`self.SetActorHiddenInGame` _item_2 false)
    (`self.K2_AttachRootComponentTo` _item_2 (`self.Mesh`) (`KismetStringLibrary.Conv_StringToName` (`KismetStringLibrary.Concat_StrStr` "ice" (`KismetStringLibrary.Conv_IntToString` _index_2))) "KeepRelativeOffset" true))
  ;[1 1 1] electro setup
  (for _index_3 (range 1 (+ (`self.numElectro`) 1))
    (bind _returnvalue_6 (`GameplayStatics.SpawnEmitterAttached` "/Game/Particles/Beam/Elecrify.Elecrify" (`self.Mesh`) (`KismetStringLibrary.Conv_StringToName` (`KismetStringLibrary.Concat_StrStr` "elect" (`KismetStringLibrary.Conv_IntToString` _index_3))) (0.0 0.0 0.0) (struct) "SnapToTarget" false))
    (bind _returnvalue_7 (`KismetArrayLibrary.Array_Add` _elctroeffect _returnvalue_6))
    (`SceneComponent.SetWorldScale3D` (`KismetArrayLibrary.Array_Get` _elctroeffect _returnvalue_7) (`self.startingScale`))))

(fn `SystemShock`
  (`KismetSystemLibrary.PrintString` "Shock")
  (set `self.SystemShocked` true)
  (set `self.delyReset` 5.0)
  (for _array_element (`self.elctroEffect`)
    (`ActorComponent.Activate` _array_element false)))

(fn `TakeDamage`
  (params (Amount :type "Float (double-precision)"))
  (`KismetSystemLibrary.PrintString` (`KismetStringLibrary.Concat_StrStr` "Malfiuntion: " (`KismetStringLibrary.Conv_DoubleToString` Amount)))
  (set `self.Damage` (+ Amount (`self.Damage`))))

(fn `Update`
  (bind _currentnumsparkstoset (`self.currentNumSparksToSet`))
  (bind _delyreset (`self.delyReset`))
  (`self.calculateWalkSpeed`)
  ;[1 1 1] Electro System
  (if (`self.SystemShocked`)
    (set `self.delyReset` (- _delyreset 0.5))
    (if (< _delyreset 0.0)
      (`self.Reset System`)))
  ;[1 1 1] Spark System
  (if (!= 0.0 (`self.Damage`))
    (`KismetSystemLibrary.PrintString` (`KismetStringLibrary.Concat_StrStr` "Total Damage:  " (`KismetStringLibrary.Conv_DoubleToString` (`self.Damage`))))
    (`self.calculateNumSparksToActivate`)
    (if (!= 0 _currentnumsparkstoset)
      (`KismetSystemLibrary.PrintString` (`KismetStringLibrary.Concat_StrStr` "Activate num Sparks: " (`KismetStringLibrary.Conv_IntToString` _currentnumsparkstoset)))
      (`self.Activate Sparks`))))

(fn `UserConstructionScript`
  (set `self.maxSparks` 5)
  (set `self.totalDamageCanTake` 100.0)
  (set `self.currentNumSparksToSet` 0)
  (set `self.numIce` 11)
  (set `self.scaleIceAmount` 1.0)
  (set `self.icescaleCap` 4.0)
  (set `self.numElectro` 9)
  (set `self.delyReset` 5.0)
  (set `self.SystemShocked` true)
  (set `self.Damage` 0.0)
  (set `self.originalIceScale` (0.5 0.5 0.25))
  (set `self.startingScale` (1.0 1.0 1.0)))