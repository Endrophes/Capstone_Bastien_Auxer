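; Standard robot enemy bot that spawns a gun on start, attacks when it finds an enemy, and plays a death animation when killed.
; BeginPlay spawns the AttackGun class, attaches it collision-free to the mesh's gun socket, and binds EnemyFound to Attack.
; Tick runs Update while alive, then once on death stops movement and stores its rotation.
; The construction script extends the parent's, tuning effect counts and speed before SetUp.
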(event `self.ReceiveBeginPlay`
  (`self.Get gun`)
  (add `self.EnemyFound` (delegate `EnemyFound_Event`)))

(event `EnemyFound_Event`
  (`self.Attack`))

(event `self.ReceiveTick`
  (params (DeltaSeconds :type "Float (single-precision)"))
  (if (`self.Alive`)
    (`self.Update`)
    (elif (not (`self.Dead`))
      (`ActorComponent.Deactivate` (`self.CharacterMovement`))
      (`SkeletalMeshComponent.PlayAnimation` (`self.Mesh`) "/Game/Blueprints/bot/Robots/Standard/RobotStandard_Anim_Death.RobotStandard_Anim_Death" false)
      (set `self.Dead` true)
      (set `self.Last Rotation` (`self.K2_GetActorRotation`)))))

(fn `Get gun`
  (bind _returnvalue (`|SpawnActorFromClass` "/Game/Blueprints/Guns/attackGun.AttackGun_C" (`self.GetTransform`) true))
  (set `self.gun` _returnvalue)
  (if (`KismetSystemLibrary.IsValid` (`self.gun`))
    (`self.SetActorEnableCollision` (`self.gun`) false)
    (`self.K2_AttachRootComponentTo` (`self.gun`) (`self.Mesh`) "gun" "SnapToTarget" true)
    (else
      (`KismetSystemLibrary.PrintString` "Failed to spawn"))))

(fn `UserConstructionScript`
  (`parent.UserConstructionScript`)
  (set `self.maxSparks` 5)
  (set `self.NumIce` 7)
  (set `self.numElectro` 8)
  (`self.SetUp`)
  (set `self.speedVar` 10.0))